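; A moving target actor for a microgame that takes hits until it is destroyed.
; Each tick it moves along its normalized Direction at Speed without sweeping, and a looping timer reverses the direction every MovementDuration, so it shuttles back and forth.
; The Hit event decrements HitPoints and plays a sound, or at zero spawns an explosion with sound and destroys the actor.
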(event `self.ReceiveBeginPlay`
  ;[0.3343 0.7766 1] Flip Direction
  (`KismetSystemLibrary.K2_SetTimerDelegate` (delegate `CustomEvent_FlipDirection`) (`self.MovementDuration`) true))

(event `CustomEvent_FlipDirection`
  ;[0.3343 0.7766 1] Flip Direction
  (set `self.Direction` (* (`self.Direction`) -1.0)))

(event `self.ReceiveTick`
  (params (DeltaSeconds :type "Float (single-precision)"))
  ;[0.4354 1 0.506] Target Movement
  (`self.K2_AddActorWorldOffset` (* (`KismetMathLibrary.Normal` (`self.Direction`)) (`self.Speed`))))

(event `self.ReceiveHit`
  (params (MyComp :type "PrimitiveComponent Object Reference") (Other :type "Actor Object Reference") (OtherComp :type "PrimitiveComponent Object Reference") (bSelfMoved :type Boolean) (HitLocation :type "Vector Structure") (HitNormal :type "Vector Structure") (NormalImpulse :type "Vector Structure") (Hit :type "HitResult Structure (by ref)"))
  ;[1 0.1979 0.1979] Hit & Destroy
  (set `self.HitPoints` (- (`self.HitPoints`) 1))
  (if (<= (`self.HitPoints`) 0)
    (`GameplayStatics.SpawnEmitterAtLocation` "/Game/StarterContent/Particles/P_Explosion.P_Explosion" HitLocation)
    (`GameplayStatics.PlaySoundAtLocation` "/Game/StarterContent/Audio/Explosion02.Explosion02" HitLocation (struct) 1.0 1.0 0.0 null null null null)
    (`self.K2_DestroyActor`)
    (else
      (`GameplayStatics.PlaySoundAtLocation` null HitLocation (struct) 1.0 1.0 0.0 null null null null))))

(fn `UserConstructionScript`)