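; BP_Key is a pickup key for a microgame that appears once no BP_MovingTarget actors remain in the level.
; Each Tick it searches for targets, sets the key mesh's visibility, and fires a one-time explosion and sound when none are left.
; Player overlap with the capsule sets HasKey on BP_FirstPersonCharacter, plays a sound and destroys the key, with no check on visibility.
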(event `self.ReceiveBeginPlay`
  ;[1 0.9645 0.452] Setup
  (bind _asbp_first_person_character (cast `/Game/FirstPerson/Blueprints/BP_FirstPersonCharacter` (`GameplayStatics.GetPlayerCharacter` 0)))
  (set `self.As BP First Person Character` _asbp_first_person_character))

(event `self.ReceiveTick`
  (params (DeltaSeconds :type "Float (single-precision)"))
  (bind _returnvalue (`SceneComponent.K2_GetComponentLocation` (`self.SM_Key`)))
  ;[1 0.6931 0.3694] Key - Visibility
  (bind _outactors (`GameplayStatics.GetAllActorsOfClass` "/Game/MicroGames/BP_MovingTarget.BP_MovingTarget_C"))
  (bind _returnvalue_2 (`KismetArrayLibrary.Array_Add` _outactors))
  (bind _returnvalue_3 (<= _returnvalue_2 0))
  (`SceneComponent.SetVisibility` (`self.SM_Key`) _returnvalue_3 true)
  ;[1 0.5955 0.5256] Key - Effects
  (if _returnvalue_3
    (`/Engine/EditorBlueprintResources/StandardMacros.DoOnce` false
      (:`Completed`
        (`GameplayStatics.SpawnEmitterAtLocation` "/Game/StarterContent/Particles/P_Explosion.P_Explosion" _returnvalue)
        (`GameplayStatics.PlaySoundAtLocation` "/Engine/EditorSounds/Notifications/CompileSuccess.CompileSuccess" _returnvalue (struct) 1.0 1.0 0.0 null null null null)))))

(event `self.Capsule_Collider.OnComponentBeginOverlap`
  (params (OverlappedComponent :type "PrimitiveComponent Object Reference") (OtherActor :type "Actor Object Reference") (OtherComp :type "PrimitiveComponent Object Reference") (OtherBodyIndex :type Integer) (bFromSweep :type Boolean) (SweepResult :type "HitResult Structure (by ref)"))
  ;[1 0.6263 0.9512] Key - Pickup
  (if (== OtherActor (`self.As BP First Person Character`))
    (set `/Game/FirstPerson/Blueprints/BP_FirstPersonCharacter.HasKey` true (`self.As BP First Person Character`))
    (`GameplayStatics.PlaySoundAtLocation` "/Engine/VREditor/Sounds/UI/Camera_Shutter.Camera_Shutter" (`self.K2_GetActorLocation`) (struct) 1.0 1.0 0.0 null null null null)
    (`self.K2_DestroyActor`)))

(fn `UserConstructionScript`)